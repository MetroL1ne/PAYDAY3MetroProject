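; Spawn group actor for the Vault Holdout custom heist mod that creates a batch of BP_SpawnPawn actors and keeps them in PawnSpawnArray.
; The SpawnPawns event spawns SpawnPawnAmount pawns using the StaticMesh's relative transform and attaches each to itself with relative rules.
; A SpawnPawns function instead takes a count and spawns owned, unattached pawns at the actor's transform.
; Nothing here triggers spawning on its own.
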(event Custom|Spawn%20Pawns
  (bind _self self)
  (for _index (range 0 (- (Variables|Default|GetSpawn%20Pawn%20Amount) 1))
    (bind _returnvalue (Game|SpawnActorfromClass "/Game/Mods/MetroMods/VaultHoldoutCustomHeist/MapUnits/Blueprints/BP_SpawnPawn.BP_SpawnPawn_C" (Transformation|GetRelativeTransform (Variables|Default|GetStaticMesh _self)) "Undefined" 0 0))
    (Transformation|AttachActorToActor _returnvalue _self "None" "KeepRelative" "KeepRelative" "KeepRelative" true)
    (Utilities|Array|Add (Variables|Default|GetPawnSpawnArray) _returnvalue)))

(event EventBeginPlay)

(event Collision|EventActorBeginOverlap
  (params (OtherActor :type Actor%20Object%20Reference)))

(event EventTick
  (params (DeltaSeconds :type Float%20%28single-precision%29)))

(fn ConstructionScript)

(fn SpawnPawns
  (params (Amount%20of%20spawn%20pawns :type Integer))
  (bind _array (Utilities|Array|MakeArray 0))
  (bind _self self)
  (for _index (range 0 (- Amount%20of%20spawn%20pawns 1))
    (bind _returnvalue (Game|SpawnActorfromClass "/Game/Mods/MetroMods/VaultHoldoutCustomHeist/MapUnits/Blueprints/BP_SpawnPawn.BP_SpawnPawn_C" (Transformation|GetActorTransform _self) "Undefined" _self 0))
    (Utilities|Array|Add _array _returnvalue)
    (Variables|Default|SetPawnSpawnArray _array)))