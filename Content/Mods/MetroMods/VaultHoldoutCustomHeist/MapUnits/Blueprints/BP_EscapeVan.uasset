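; Map unit for the Vault Holdout custom heist that spawns and controls an escape van.
; SpawnVan creates a BP_EscapeVan at this actor's transform and registers it through SetEscapeVan.
; SetandDriveEscapeVanRoute sends that van along start and end splines, with optional teleport to the path start, then calls the route-completed notification.
; ToggleDoors flips the spawned van's door-open state with a FlipFlop.
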(event Custom|Toggle%20Doors
  (bind _isa (Utilities|FlowControl|FlipFlop)
    (:A
      _)
    (:B
      _))
  (Variables|/Game/Vehicle/_Mockup/Escape/BP_EscapeVan.BP_EscapeVan_C|SetisDoorOpen (stale Custom|Spawn%20Van _returnvalue) _isa))

(event Custom|Set%20and%20Drive%20Escape%20Van%20Route
  (Class|SBZTrafficFunctionLibrary|SetandDriveEscapeVanRoute (stale Custom|Spawn%20Van _returnvalue) (Variables|Default|GetStart%20Spline) (Variables|Default|GetEnd%20Spline) (Variables|Default|GetTeleport%20to%20%20Path%20Start))
  (Default|CallEscapeVanRouteCompleted))

(event Custom|Spawn%20Van
  (bind _returnvalue (Game|SpawnActorfromClass "/Game/Vehicle/_Mockup/Escape/BP_EscapeVan.BP_EscapeVan_C" (Transformation|GetActorTransform self) "Undefined" 0 0))
  (Class|SBZTrafficFunctionLibrary|SetEscapeVan _returnvalue))

(event Collision|EventActorBeginOverlap
  (params (OtherActor :type Actor%20Object%20Reference)))

(event EventTick
  (params (DeltaSeconds :type Float%20%28single-precision%29)))

(fn ConstructionScript)