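; BP_SpawnStaticVehicle is a map placement actor that spawns a static vehicle at its own transform on BeginPlay.
; An enum selects the vehicle class (sedan, trucks, SUV or van), though the Sedan 2 option has no class assigned.
; The spawned SBZStaticVehicle receives the HasAlarm setting and a random seed.
; Logic to resize a placeholder cube by vehicle type exists but is disconnected from the empty construction script.
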(event EventBeginPlay
  (switch Utilities|FlowControl|Switch|SwitchonPD3Vehicles (Variables|Default|GetNewVar_0)
    (:NewEnumerator0
      (Variables|Default|SetVehicle "/Game/Vehicle/Civilian/Car/BP_StaticVehicle_Sedan_Civilian.BP_StaticVehicle_Sedan_Civilian_C"))
    (:NewEnumerator1
      (Variables|Default|SetVehicle 0))
    (:NewEnumerator2
      (Variables|Default|SetVehicle "/Game/Vehicle/Civilian/Truck/Veh_Delivery_Truck_01/BP_StaticVehicle_Delivery_Truck_01.BP_StaticVehicle_Delivery_Truck_01_C"))
    (:NewEnumerator3
      (Variables|Default|SetVehicle "/Game/Vehicle/Civilian/Truck/Veh_Med_Truck_01/BP_StaticVehicle_MediumTruck.BP_StaticVehicle_MediumTruck_C"))
    (:NewEnumerator4
      (Variables|Default|SetVehicle "/Game/Vehicle/Civilian/Suv/BP_StaticVehicle_Suv.BP_StaticVehicle_Suv_C"))
    (:NewEnumerator5
      (Variables|Default|SetVehicle "/Game/Vehicle/Civilian/Van/Veh_Van_01/BP_StaticVehicle_Van_01.BP_StaticVehicle_Van_01_C")))
  (bind _returnvalue (Game|SpawnActorfromClass (Variables|Default|GetVehicle) (Transformation|GetActorTransform self) "Undefined" 0 0))
  (bind _assbzstatic_vehicle (Utilities|Casting|CastToSBZStaticVehicle _returnvalue))
  (Variables|/Script/Starbreeze.SBZStaticVehicle|SetbHasAlarm _assbzstatic_vehicle (Variables|Default|GetHas%20Alarm))
  (Variables|/Script/Starbreeze.SBZStaticVehicle|SetSeed _assbzstatic_vehicle (Math|Random|RandomIntegerinRange -10000 10000)))

(fn ConstructionScript)